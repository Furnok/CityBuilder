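; Grid cell for a city-builder that tracks its occupying structure and four neighbours.
; On occupation it adds clamped Satisfaction to game-instance stats for House adjacency to satisfaction-giving structures, then refreshes the HUD; clearing subtracts only the bonus stored on that cell, which Houses leave at zero.
; Neighbour checks are nested, so a missing neighbour ends the search.
; Init respawns a House, Farm, Park or Road from given state, registering roads with BP_RoadManager.
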(event `SetOccupied`
  (params (Type :type "/Game/Game/Blueprints/Grid/E_BuildingType Enum" :default "NewEnumerator3") (Actor :type "Actor Object Reference") (Name :type String))
  (bind _neighbournorth (`self.NeighbourNorth`))
  (bind _neighboursouth (`self.NeighbourSouth`))
  (bind _neighboureast (`self.NeighbourEast`))
  (bind _neighbourwest (`self.NeighbourWest`))
  (bind _neighboursouth_2 (`self.NeighbourSouth`))
  (bind (_infoneighbour_name _infoneighbour_description _infoneighbour_level _infoneighbour_levelmax _infoneighbour_population _infoneighbour_radius _infoneighbour_satisfaction) (break `/Game/Game/Blueprints/DataAsset/S_Info` (`self.InfoNeighbour`)))
  (bind _neighbournorth_2 (`self.NeighbourNorth`))
  (bind _neighboureast_2 (`self.NeighbourEast`))
  (bind _neighbourwest_2 (`self.NeighbourWest`))
  (bind _name (`/Game/Game/Blueprints/Grid/BP_GridCell.Name` _neighboursouth_2))
  (bind _name_2 (`/Game/Game/Blueprints/Grid/BP_GridCell.Name` _neighboureast))
  (bind _name_3 (`/Game/Game/Blueprints/Grid/BP_GridCell.Name` _neighbourwest))
  (bind _name_4 (`/Game/Game/Blueprints/Grid/BP_GridCell.Name` _neighbournorth_2))
  (set `self.IsOccupied` true)
  (set `self.OccupingType` Type)
  (bind _output_get (set `self.OccupingActor` Actor))
  (set `self.Name` Name)
  (set `self.Satisfaction` 0)
  (`KismetSystemLibrary.Delay` 0.1)
  (bind _asbp_placable_structure (cast `/Game/Game/Blueprints/Structures/BP_PlacableStructure` _output_get))
  (bind (_info_name _info_description _info_level _info_levelmax _info_population _info_radius _info_satisfaction) (break `/Game/Game/Blueprints/DataAsset/S_Info` (`/Game/Game/Blueprints/Structures/BP_PlacableStructure.Info` _asbp_placable_structure)))
  (if (!= _info_satisfaction 0)
    (`/Engine/EditorBlueprintResources/StandardMacros.IsValid` _neighbournorth
      (:`Is Valid`
        (if (`KismetStringLibrary.EqualEqual_StrStr` (`/Game/Game/Blueprints/Grid/BP_GridCell.Name` _neighbournorth) "House")
          (bind _asbp_player_game_instance (cast `/Game/Game/Saves/BP_PlayerGameInstance` (`GameplayStatics.GetGameInstance`) :!label _label))
          (bind (_stats_money _stats_satisfaction _stats_population _stats_populationmax) (break `/Game/Game/Blueprints/DataAsset/S_StatsStart` (`/Game/Game/Saves/BP_PlayerGameInstance.Stats` _asbp_player_game_instance)))
          (set `/Game/Game/Saves/BP_PlayerGameInstance.Stats` (make `/Game/Game/Blueprints/DataAsset/S_StatsStart` _stats_money (`KismetMathLibrary.Clamp` (+ _stats_satisfaction _info_satisfaction) 0 100) _stats_population _stats_populationmax) _asbp_player_game_instance)
          (set `self.Satisfaction` _info_satisfaction)
          (bind _asbp_uihud (cast `/Game/Game/Blueprints/HUD/BP_UIHUD` (`PlayerController.GetHUD` (`GameplayStatics.GetPlayerController` 0))))
          (`/Game/Game/UI/WB_MainGame.Initialisation UI` (`/Game/Game/Blueprints/HUD/BP_UIHUD.MainGame` _asbp_uihud))
          (else
            (`/Engine/EditorBlueprintResources/StandardMacros.IsValid` _neighboursouth
              (:`Is Valid`
                (if (`KismetStringLibrary.EqualEqual_StrStr` (`/Game/Game/Blueprints/Grid/BP_GridCell.Name` _neighboursouth) "House")
                  (goto _label)
                  (else
                    (`/Engine/EditorBlueprintResources/StandardMacros.IsValid` _neighboureast_2
                      (:`Is Valid`
                        (if (`KismetStringLibrary.EqualEqual_StrStr` (`/Game/Game/Blueprints/Grid/BP_GridCell.Name` _neighboureast_2) "House")
                          (goto _label)
                          (else
                            (`/Engine/EditorBlueprintResources/StandardMacros.IsValid` _neighbourwest_2
                              (:`Is Valid`
                                (if (`KismetStringLibrary.EqualEqual_StrStr` (`/Game/Game/Blueprints/Grid/BP_GridCell.Name` _neighbourwest_2) "House")
                                  (goto _label))))))))))))))))
    (elif (`KismetStringLibrary.EqualEqual_StrStr` _info_name "House")
      (`/Engine/EditorBlueprintResources/StandardMacros.IsValid` _neighbournorth_2
        (:`Is Valid`
          (if (or (`KismetStringLibrary.EqualEqual_StrStr` _name_4 "Farm") (`KismetStringLibrary.EqualEqual_StrStr` _name_4 "Park"))
            (bind _asbp_placable_structure_2 (cast `/Game/Game/Blueprints/Structures/BP_PlacableStructure` (`/Game/Game/Blueprints/Grid/BP_GridCell.OccupingActor` _neighbournorth_2)))
            (set `self.InfoNeighbour` (`/Game/Game/Blueprints/Structures/BP_PlacableStructure.Info` _asbp_placable_structure_2))
            (bind _asbp_player_game_instance_2 (cast `/Game/Game/Saves/BP_PlayerGameInstance` (`GameplayStatics.GetGameInstance`) :!label _label_2))
            (bind (_stats_money_2 _stats_satisfaction_2 _stats_population_2 _stats_populationmax_2) (break `/Game/Game/Blueprints/DataAsset/S_StatsStart` (`/Game/Game/Saves/BP_PlayerGameInstance.Stats` _asbp_player_game_instance_2)))
            (set `/Game/Game/Saves/BP_PlayerGameInstance.Stats` (make `/Game/Game/Blueprints/DataAsset/S_StatsStart` _stats_money_2 (`KismetMathLibrary.Clamp` (+ _stats_satisfaction_2 _infoneighbour_satisfaction) 0 100) _stats_population_2 _stats_populationmax_2) _asbp_player_game_instance_2)
            (set `self.Satisfaction` 0)
            (bind _asbp_uihud_2 (cast `/Game/Game/Blueprints/HUD/BP_UIHUD` (`PlayerController.GetHUD` (`GameplayStatics.GetPlayerController` 0))))
            (`/Game/Game/UI/WB_MainGame.Initialisation UI` (`/Game/Game/Blueprints/HUD/BP_UIHUD.MainGame` _asbp_uihud_2))
            (else
              (`/Engine/EditorBlueprintResources/StandardMacros.IsValid` _neighboursouth_2
                (:`Is Valid`
                  (if (or (`KismetStringLibrary.EqualEqual_StrStr` _name "Farm") (`KismetStringLibrary.EqualEqual_StrStr` _name "Park"))
                    (bind _asbp_placable_structure_3 (cast `/Game/Game/Blueprints/Structures/BP_PlacableStructure` (`/Game/Game/Blueprints/Grid/BP_GridCell.OccupingActor` _neighboursouth_2)))
                    (set `self.InfoNeighbour` (`/Game/Game/Blueprints/Structures/BP_PlacableStructure.Info` _asbp_placable_structure_3))
                    (goto _label_2)
                    (else
                      (`/Engine/EditorBlueprintResources/StandardMacros.IsValid` _neighboureast
                        (:`Is Valid`
                          (if (or (`KismetStringLibrary.EqualEqual_StrStr` _name_2 "Farm") (`KismetStringLibrary.EqualEqual_StrStr` _name_2 "Park"))
                            (bind _asbp_placable_structure_4 (cast `/Game/Game/Blueprints/Structures/BP_PlacableStructure` (`/Game/Game/Blueprints/Grid/BP_GridCell.OccupingActor` _neighboureast)))
                            (set `self.InfoNeighbour` (`/Game/Game/Blueprints/Structures/BP_PlacableStructure.Info` _asbp_placable_structure_4))
                            (goto _label_2)
                            (else
                              (`/Engine/EditorBlueprintResources/StandardMacros.IsValid` _neighbourwest
                                (:`Is Valid`
                                  (if (or (`KismetStringLibrary.EqualEqual_StrStr` _name_3 "Farm") (`KismetStringLibrary.EqualEqual_StrStr` _name_3 "Park"))
                                    (bind _asbp_placable_structure_5 (cast `/Game/Game/Blueprints/Structures/BP_PlacableStructure` (`/Game/Game/Blueprints/Grid/BP_GridCell.OccupingActor` _neighbourwest)))
                                    (set `self.InfoNeighbour` (`/Game/Game/Blueprints/Structures/BP_PlacableStructure.Info` _asbp_placable_structure_5))
                                    (goto _label_2)))))))))))))))))))

(event `SetUnOccupied`
  (set `self.IsOccupied` false)
  (set `self.OccupingType` "NewEnumerator3")
  (set `self.OccupingActor` null)
  (set `self.Name` "")
  (if (!= (`self.Satisfaction`) 0)
    (`KismetSystemLibrary.Delay` 0.1)
    (bind _asbp_player_game_instance (cast `/Game/Game/Saves/BP_PlayerGameInstance` (`GameplayStatics.GetGameInstance`)))
    (bind (_stats_money _stats_satisfaction _stats_population _stats_populationmax) (break `/Game/Game/Blueprints/DataAsset/S_StatsStart` (`/Game/Game/Saves/BP_PlayerGameInstance.Stats` _asbp_player_game_instance)))
    (set `/Game/Game/Saves/BP_PlayerGameInstance.Stats` (make `/Game/Game/Blueprints/DataAsset/S_StatsStart` _stats_money (`KismetMathLibrary.Clamp` (- _stats_satisfaction (`self.Satisfaction`)) 0 100) _stats_population _stats_populationmax) _asbp_player_game_instance)
    (bind _asbp_uihud (cast `/Game/Game/Blueprints/HUD/BP_UIHUD` (`PlayerController.GetHUD` (`GameplayStatics.GetPlayerController` 0))))
    (`/Game/Game/UI/WB_MainGame.Initialisation UI` (`/Game/Game/Blueprints/HUD/BP_UIHUD.MainGame` _asbp_uihud))
    (set `self.Satisfaction` 0)))

(event `Init`
  (params (Occupied :type Boolean) (Type :type "/Game/Game/Blueprints/Grid/E_BuildingType Enum" :default "NewEnumerator3") (Actor :type "Actor Object Reference") (Name :type String) (Info :type "/Game/Game/Blueprints/DataAsset/S_Info Structure"))
  (bind (_returnvalue_location _returnvalue_rotation _returnvalue_scale) (`KismetMathLibrary.BreakTransform` (`self.GetTransform`)))
  (bind (_returnvalue_location_2 _returnvalue_rotation_2 _returnvalue_scale_2) (`KismetMathLibrary.BreakTransform` (`self.GetTransform`)))
  (bind (_returnvalue_location_3 _returnvalue_rotation_3 _returnvalue_scale_3) (`KismetMathLibrary.BreakTransform` (`self.GetTransform`)))
  (bind (_returnvalue_location_4 _returnvalue_rotation_4 _returnvalue_scale_4) (`KismetMathLibrary.BreakTransform` (`self.GetTransform`)))
  (bind (_info_name _info_description _info_level _info_levelmax _info_population _info_radius _info_satisfaction _info_money _info_cost _info_coeffupgrade _info_coeff2 _info_upgrade _info_rotation) (break `/Game/Game/Blueprints/DataAsset/S_Info` (`self.Info`)))
  (set `self.IsOccupied` Occupied)
  (set `self.OccupingType` Type)
  (set `self.OccupingActor` Actor)
  (bind _output_get (set `self.Name` Name))
  (set `self.Info` Info)
  (if (`KismetStringLibrary.EqualEqual_StrStr` _output_get "House")
    (bind _returnvalue (`|SpawnActorFromClass` "/Game/Game/Blueprints/Structures/BP_House.BP_House_C" (`KismetMathLibrary.MakeTransform` (+ _returnvalue_location (0.0 0.0 50.0)) _info_rotation _returnvalue_scale) "AlwaysSpawn" "MultiplyWithRoot" null null))
    (bind _asbp_placable_structure (cast `/Game/Game/Blueprints/Structures/BP_PlacableStructure` _returnvalue))
    (set `/Game/Game/Blueprints/Structures/BP_PlacableStructure.GridCell` self _asbp_placable_structure)
    (`/Game/Game/Blueprints/Structures/BP_PlacableStructure.Initialise` _asbp_placable_structure "/Game/Game/Blueprints/DataAsset/Data/DataAsset_House.DataAsset_House" (`self.Info`) true)
    (set `self.OccupingActor` _asbp_placable_structure)
    (elif (`KismetStringLibrary.EqualEqual_StrStr` _output_get "Farm")
      (bind _returnvalue_2 (`|SpawnActorFromClass` "/Game/Game/Blueprints/Structures/BP_Farm.BP_Farm_C" (`KismetMathLibrary.MakeTransform` (+ _returnvalue_location_3 (0.0 0.0 50.0)) _info_rotation _returnvalue_scale_3) "AlwaysSpawn" "MultiplyWithRoot" null null))
      (bind _asbp_placable_structure_2 (cast `/Game/Game/Blueprints/Structures/BP_PlacableStructure` _returnvalue_2))
      (set `/Game/Game/Blueprints/Structures/BP_PlacableStructure.GridCell` self _asbp_placable_structure_2)
      (`/Game/Game/Blueprints/Structures/BP_PlacableStructure.Initialise` _asbp_placable_structure_2 "/Game/Game/Blueprints/DataAsset/Data/DataAsset_Farm.DataAsset_Farm" (`self.Info`) true)
      (set `self.OccupingActor` _asbp_placable_structure_2)
      (elif (`KismetStringLibrary.EqualEqual_StrStr` _output_get "Park")
        (bind _returnvalue_3 (`|SpawnActorFromClass` "/Game/Game/Blueprints/Structures/BP_Park.BP_Park_C" (`KismetMathLibrary.MakeTransform` (+ _returnvalue_location_2 (0.0 0.0 50.0)) _info_rotation _returnvalue_scale_2) "AlwaysSpawn" "MultiplyWithRoot" null null))
        (bind _asbp_placable_structure_3 (cast `/Game/Game/Blueprints/Structures/BP_PlacableStructure` _returnvalue_3))
        (set `/Game/Game/Blueprints/Structures/BP_PlacableStructure.GridCell` self _asbp_placable_structure_3)
        (`/Game/Game/Blueprints/Structures/BP_PlacableStructure.Initialise` _asbp_placable_structure_3 "/Game/Game/Blueprints/DataAsset/Data/DataAsset_Park.DataAsset_Park" (`self.Info`) true)
        (set `self.OccupingActor` _asbp_placable_structure_3)
        (elif (`KismetStringLibrary.EqualEqual_StrStr` _output_get "Road")
          (bind _returnvalue_4 (`|SpawnActorFromClass` "/Game/Game/Blueprints/Structures/BP_Road.BP_Road_C" (`KismetMathLibrary.MakeTransform` (+ _returnvalue_location_4 (0.0 0.0 50.0)) _info_rotation _returnvalue_scale_4) "AlwaysSpawn" "MultiplyWithRoot" null null))
          (bind _asbp_placable_structure_4 (cast `/Game/Game/Blueprints/Structures/BP_PlacableStructure` _returnvalue_4))
          (set `/Game/Game/Blueprints/Structures/BP_PlacableStructure.GridCell` self _asbp_placable_structure_4)
          (`/Game/Game/Blueprints/Structures/BP_PlacableStructure.Initialise` _asbp_placable_structure_4 "/Game/Game/Blueprints/DataAsset/Data/DataAsset_Road.DataAsset_Road" (`self.Info`) true)
          (set `self.OccupingActor` _asbp_placable_structure_4)
          (bind _returnvalue_5 (`GameplayStatics.GetActorOfClass` "/Game/Game/Blueprints/Road/BP_RoadManager.BP_RoadManager_C"))
          (`/Game/Game/Blueprints/Road/BP_RoadManager.AddRoadTile` _returnvalue_5 _returnvalue_4))))))

(fn `UserConstructionScript`)

(fn `Visibility`
  (params (Visibility :type Boolean))
  (bind _defaultsceneroot (`self.DefaultSceneRoot`))
  (if Visibility
    (`SceneComponent.SetVisibility` _defaultsceneroot true true)
    (else
      (`SceneComponent.SetVisibility` _defaultsceneroot false true))))