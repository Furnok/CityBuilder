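; BP_Grid builds a centred square grid of attached BP_GridCell actors that track what occupies them.
; On BeginPlay, the game instance's Create flag selects a fresh grid or one restored from its saved occupancy arrays.
; It then links each cell to its four neighbours by index in the flat array.
; Helpers find the closest cell or position by linear distance search and toggle visibility on every cell.
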(event `self.ReceiveBeginPlay`
  (bind _asbp_player_game_instance (cast `/Game/Game/Saves/BP_PlayerGameInstance` (`GameplayStatics.GetGameInstance`)))
  (if (`/Game/Game/Saves/BP_PlayerGameInstance.Create` _asbp_player_game_instance)
    (`self.PopulateGrid`)
    (else
      (`self.LoadGrid`)))
  (`self.PopulateGridCellNeighbours`))

(fn `GetClosestGridCell`
  (params (InPosition :type "Vector Structure"))
  (returns (OutputCell :type "/Game/Game/Blueprints/Grid/BP_GridCell Object Reference"))
  (locals (ClosesDistance :type "Float (double-precision)") (ArrayIndex :type Integer))
  (set `local.ClosesDistance` (`KismetMathLibrary.Vector_Distance` InPosition (`self.K2_GetActorLocation` (`|GetArrayItem` (`self.GridArray`)))))
  (for (_array_element _array_index) (`self.GridArray`)
    (bind _returnvalue (`KismetMathLibrary.Vector_Distance` (`self.K2_GetActorLocation` _array_element) InPosition))
    (if (< _returnvalue (`local.ClosesDistance`))
      (set `local.ClosesDistance` _returnvalue)
      (set `local.ArrayIndex` _array_index)))
  (return (`|GetArrayItem` (`self.GridArray`) (`local.ArrayIndex`))))

(fn `GetClosestGridPosition`
  (params (InPosition :type "Vector Structure"))
  (returns (OutputVector :type "Vector Structure"))
  (locals (ClosesPosition :type "Vector Structure") (ClosesDistance :type "Float (double-precision)"))
  (bind _returnvalue (`self.K2_GetActorLocation` (`|GetArrayItem` (`self.GridArray`))))
  (set `local.ClosesPosition` _returnvalue)
  (set `local.ClosesDistance` (`KismetMathLibrary.Vector_Distance` InPosition _returnvalue))
  (for _array_element (`self.GridArray`)
    (bind _returnvalue_2 (`self.K2_GetActorLocation` _array_element))
    (bind _returnvalue_3 (`KismetMathLibrary.Vector_Distance` _returnvalue_2 InPosition))
    (if (< _returnvalue_3 (`local.ClosesDistance`))
      (set `local.ClosesPosition` _returnvalue_2)
      (set `local.ClosesDistance` _returnvalue_3)))
  (return (`local.ClosesPosition`)))

(fn `LoadGrid`
  (locals (WorldOffset :type "Float (double-precision)"))
  (bind _worldgridsize (`self.WorldGridSize`))
  (bind _worldgridsize_2 (`self.WorldGridSize`))
  (bind _worldoffset (`local.WorldOffset`))
  (`KismetArrayLibrary.Array_Clear` (`self.GridArray`))
  (set `local.WorldOffset` (- (* (* (`self.GridSize`) _worldgridsize) 0.5) (* _worldgridsize 0.5)))
  (for _index (range (`self.GridSize`))
    (for _index_2 (range (`self.GridSize`))
      (bind _returnvalue (`|SpawnActorFromClass` "/Game/Game/Blueprints/Grid/BP_GridCell.BP_GridCell_C" (`KismetMathLibrary.MakeTransform` (`KismetMathLibrary.MakeVector` (- (* _index_2 _worldgridsize_2) _worldoffset) (- (* _worldgridsize_2 _index) _worldoffset))) "AlwaysSpawn" "MultiplyWithRoot" null null))
      (`KismetArrayLibrary.Array_Add` (`self.GridArray`) _returnvalue)
      (`self.K2_AttachToActor` _returnvalue self "None" "KeepRelative" "KeepRelative" "KeepRelative" true)))
  (bind _asbp_player_game_instance (cast `/Game/Game/Saves/BP_PlayerGameInstance` (`GameplayStatics.GetGameInstance`)))
  (for (_array_element _array_index) (`self.GridArray`)
    (`/Game/Game/Blueprints/Grid/BP_GridCell.Init` _array_element (`|GetArrayItem` (`/Game/Game/Saves/BP_PlayerGameInstance.IsOccupied` _asbp_player_game_instance) _array_index) (`|GetArrayItem` (`/Game/Game/Saves/BP_PlayerGameInstance.OccupingType` _asbp_player_game_instance) _array_index) (`|GetArrayItem` (`/Game/Game/Saves/BP_PlayerGameInstance.OccupingActor` _asbp_player_game_instance) _array_index) (`|GetArrayItem` (`/Game/Game/Saves/BP_PlayerGameInstance.Name` _asbp_player_game_instance) _array_index) (`|GetArrayItem` (`/Game/Game/Saves/BP_PlayerGameInstance.Info` _asbp_player_game_instance) _array_index))))

(fn `PopulateGrid`
  (locals (WorldOffset :type "Float (double-precision)"))
  (bind _worldgridsize (`self.WorldGridSize`))
  (bind _worldgridsize_2 (`self.WorldGridSize`))
  (bind _worldoffset (`local.WorldOffset`))
  (`KismetArrayLibrary.Array_Clear` (`self.GridArray`))
  (set `local.WorldOffset` (- (* (* (`self.GridSize`) _worldgridsize) 0.5) (* _worldgridsize 0.5)))
  (for _index (range (`self.GridSize`))
    (for _index_2 (range (`self.GridSize`))
      (bind _returnvalue (`|SpawnActorFromClass` "/Game/Game/Blueprints/Grid/BP_GridCell.BP_GridCell_C" (`KismetMathLibrary.MakeTransform` (`KismetMathLibrary.MakeVector` (- (* _index_2 _worldgridsize_2) _worldoffset) (- (* _worldgridsize_2 _index) _worldoffset))) "AlwaysSpawn" "MultiplyWithRoot" null null))
      (`KismetArrayLibrary.Array_Add` (`self.GridArray`) _returnvalue)
      (`self.K2_AttachToActor` _returnvalue self "None" "KeepRelative" "KeepRelative" "KeepRelative" true))))

(fn `PopulateGridCellNeighbours`
  (bind _gridarray (`self.GridArray`))
  (for (_array_element _array_index) (`self.GridArray`)
    (bind _returnvalue (- _array_index (`self.GridSize`)))
    (if (>= _returnvalue 0)
      (set `/Game/Game/Blueprints/Grid/BP_GridCell.NeighbourWest` (`|GetArrayItem` (`self.GridArray`) _returnvalue) _array_element))
    (bind _returnvalue_2 (+ _array_index (`self.GridSize`)))
    (if (< _returnvalue_2 (`KismetArrayLibrary.Array_Length` _gridarray))
      (set `/Game/Game/Blueprints/Grid/BP_GridCell.NeighbourEast` (`|GetArrayItem` _gridarray _returnvalue_2) _array_element))
    (if (not (or (== _array_index 0) (== (mod _array_index (`self.GridSize`)) 0)))
      (set `/Game/Game/Blueprints/Grid/BP_GridCell.NeighbourSouth` (`|GetArrayItem` (`self.GridArray`) (- _array_index 1)) _array_element))
    (if (not (== (mod (+ _array_index 1) (`self.GridSize`)) 0))
      (set `/Game/Game/Blueprints/Grid/BP_GridCell.NeighbourNorth` (`|GetArrayItem` (`self.GridArray`) (+ _array_index 1)) _array_element))))

(fn `UserConstructionScript`)

(fn `Visibility`
  (params (Visibility :type Boolean))
  (for _array_element (`self.GridArray`)
    (`/Game/Game/Blueprints/Grid/BP_GridCell.Visibility` _array_element Visibility)))