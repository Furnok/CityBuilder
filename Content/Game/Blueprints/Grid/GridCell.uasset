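; GridCell is a grid tile actor that records what occupies it and knows its four cardinal neighbours.
; SetOccupied stores the occupying type and actor, marks the cell occupied, then calls a debug event on the north, south, east and west neighbours.
; That debug event turns the neighbour's sphere red to visualise cells adjacent to an occupied one.
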(event `SetOccupied`
  (params (Type :type "/Game/Game/Blueprints/Grid/BuildingType Enum" :default "NewEnumerator3") (Actor :type "Actor Object Reference"))
  (set `self.IsOccupied` true)
  (set `self.OccupingType` Type)
  (set `self.OccupingActor` Actor)
  (`self.DebugShowOccupiedNeighbord` (`self.NeighbourNorth`))
  (`self.DebugShowOccupiedNeighbord` (`self.NeighbourSouth`))
  (`self.DebugShowOccupiedNeighbord` (`self.NeighbourEast`))
  (`self.DebugShowOccupiedNeighbord` (`self.NeighbourWest`)))

(event `DebugShowOccupiedNeighbord`
  (`PrimitiveComponent.SetMaterial` (`self.Sphere`) 0 "/Game/Game/Materials/Red.Red"))

(fn `UserConstructionScript`)