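; Player controller that runs grid-based building placement for a city builder, including re-placing existing structures.
; A preview actor follows a mouse line trace, snaps to BP_Grid cells and rotates in quarter turns.
; Placing checks the ploppable component's validity and money, skipping cost for Unique re-placements, then spawns the structure, occupies its cell and registers roads with BP_RoadManager.
; ResetBuilding respawns the old structure in its original cell.
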(event `self.ReceiveBeginPlay`
  (bind _returnvalue (pcsubsystem `EnhancedInputLocalPlayerSubsystem` self))
  ;[0.016 0.016 0.016] Add Inputs Mapping Context
  (`/Engine/EditorBlueprintResources/StandardMacros.IsValid` _returnvalue
    (:`Is Valid`
      (`EnhancedInputSubsystemInterface.AddMappingContext` _returnvalue "/Game/Game/Inputs/Input_Player.Input_Player" 0 (struct)))))

(event `self.ReceiveTick`
  (params (DeltaSeconds :type "Float (single-precision)"))
  (if (`self.PlacementModeEnable`)
    (`self.UpdatePlacement`))
  (bind _asbp_player_game_instance (cast `/Game/Game/Saves/BP_PlayerGameInstance` (`GameplayStatics.GetGameInstance`)))
  (bind (_stats_money _stats_satisfaction) (break `/Game/Game/Blueprints/DataAsset/S_StatsStart` (`/Game/Game/Saves/BP_PlayerGameInstance.Stats` _asbp_player_game_instance)))
  (if (<= _stats_satisfaction 0)
    _))

(event `EnhancedInput|/Game/Game/Inputs/IA_Place`
  (params (ActionValue :type Boolean) (ElapsedSeconds :type "Float (double-precision)") (TriggeredSeconds :type "Float (double-precision)") (InputAction :type "InputAction Object Reference" :default "/Game/Game/Inputs/IA_Place.IA_Place"))
  (:`Started`
    (if (`self.PlacementModeEnable`)
      (`self.SpawnBuilding`))))

(event `OnPlacementInfoUpdated`
  (params (PlaceableActorType :type "/Game/Game/Blueprints/Structures/BP_PlacableStructure Class Reference") (InPlaceableMode :type "/Game/Game/Blueprints/Grid/E_BuildingType Enum" :default "NewEnumerator3") (Unique :type Boolean) (`Struc Old` :type "/Game/Game/Blueprints/Structures/BP_PlacableStructure Object Reference"))
  (bind _placeableactor (`self.PlaceableActor`))
  (set `self.PlaceableActorType` PlaceableActorType)
  (bind _output_get (set `self.PlaceableBuildingType` InPlaceableMode))
  (set `self.Unique` Unique)
  (`/Engine/EditorBlueprintResources/StandardMacros.IsValid` `Struc Old`
    (:`Is Valid`
      (set `self.Struc Old` `Struc Old`))
    (:`Is Not Valid`
      _))
  (if (`|EnumEquality` _output_get "NewEnumerator3")
    (`self.SetPlacementModeEnable` false)
    (bind _returnvalue (`GameplayStatics.GetActorOfClass` "/Game/Game/Blueprints/Grid/BP_Grid.BP_Grid_C"))
    (`/Game/Game/Blueprints/Grid/BP_Grid.Visibility` _returnvalue false)
    (else
      (`/Engine/EditorBlueprintResources/StandardMacros.IsValid` _placeableactor
        (:`Is Valid`
          (`self.K2_DestroyActor` _placeableactor))
        (:`Is Not Valid`
          _))
      (`self.RefreshPlaceableBuilding`)
      (`self.SetPlacementModeEnable` true)
      (bind _returnvalue_2 (`GameplayStatics.GetActorOfClass` "/Game/Game/Blueprints/Grid/BP_Grid.BP_Grid_C"))
      (`/Game/Game/Blueprints/Grid/BP_Grid.Visibility` _returnvalue_2 true))))

(event `EnhancedInput|/Game/Game/Inputs/IA_RotateS`
  (params (ActionValue :type Boolean) (ElapsedSeconds :type "Float (double-precision)") (TriggeredSeconds :type "Float (double-precision)") (InputAction :type "InputAction Object Reference" :default "/Game/Game/Inputs/IA_RotateS.IA_RotateS"))
  (bind _placeableactor (`self.PlaceableActor`))
  (bind _returnvalue (`self.GetTransform` _placeableactor))
  (bind (_info_name _info_description _info_level _info_levelmax _info_population _info_radius _info_satisfaction _info_money _info_cost _info_coeffupgrade _info_coeff2 _info_upgrade) (break `/Game/Game/Blueprints/DataAsset/S_Info` (`/Game/Game/Blueprints/Structures/BP_PlacableStructure.Info` _placeableactor)))
  (:`Started`
    (if (`self.PlacementModeEnable`)
      (`self.K2_SetActorRotation` _placeableactor (`KismetMathLibrary.MakeRotator` (.roll (.rotation _returnvalue)) (.pitch (.rotation _returnvalue)) (+ (.yaw (.rotation _returnvalue)) 90.0)) false)
      (set `/Game/Game/Blueprints/Structures/BP_PlacableStructure.Info` (make `/Game/Game/Blueprints/DataAsset/S_Info` _info_name _info_description _info_level _info_levelmax _info_population _info_radius _info_satisfaction _info_money _info_cost _info_coeffupgrade _info_coeff2 _info_upgrade (`self.K2_GetActorRotation` _placeableactor)) _placeableactor))))

(fn `RefreshPlaceableBuilding`
  (bind _placeableactortype (`self.PlaceableActorType`))
  (bind _struc_old (`self.Struc Old`))
  (bind _placeableactor (`self.PlaceableActor`))
  (bind _struc_old_2 (`self.Struc Old`))
  (bind _placeableactor_2 (`self.PlaceableActor`))
  (bind _struc_old_3 (`self.Struc Old`))
  (bind (_info_name _info_description _info_level _info_levelmax _info_population _info_radius _info_satisfaction _info_money _info_cost _info_coeffupgrade _info_coeff2 _info_upgrade _info_rotation) (break `/Game/Game/Blueprints/DataAsset/S_Info` (`/Game/Game/Blueprints/Structures/BP_PlacableStructure.Info` _struc_old)))
  (`/Engine/EditorBlueprintResources/StandardMacros.IsValid` _struc_old
    (:`Is Valid`
      (bind _returnvalue (`|SpawnActorFromClass` _placeableactortype (`KismetMathLibrary.MakeTransform` (0.0 0.0 -100000.0) _info_rotation) "AlwaysSpawn" "MultiplyWithRoot" null null))
      (bind _asbp_placable_structure (cast `/Game/Game/Blueprints/Structures/BP_PlacableStructure` _returnvalue))
      (set `self.PlaceableActor` _asbp_placable_structure)
      (`/Engine/EditorBlueprintResources/StandardMacros.IsValid` _struc_old_2
        (:`Is Valid`
          (set `/Game/Game/Blueprints/Structures/BP_PlacableStructure.Structure Info` (`/Game/Game/Blueprints/Structures/BP_PlacableStructure.Structure Info` _struc_old_2) _placeableactor)
          (set `/Game/Game/Blueprints/Structures/BP_PlacableStructure.Info` (`/Game/Game/Blueprints/Structures/BP_PlacableStructure.Info` _struc_old_2) _placeableactor))
        (:`Is Not Valid`
          (bind _structure_info (`/Game/Game/Blueprints/Structures/BP_PlacableStructure.Structure Info` _returnvalue))
          (set `/Game/Game/Blueprints/Structures/BP_PlacableStructure.Structure Info` _structure_info _placeableactor)
          (set `/Game/Game/Blueprints/Structures/BP_PlacableStructure.Info` (`/Game/Game/Blueprints/DataAsset/BP_DataAsset_Structure.Info` _structure_info) _placeableactor)))
      (`AddComponent|NODE_AddPloppableComponent-0` :`self` _placeableactor))
    (:`Is Not Valid`
      (bind _returnvalue_2 (`|SpawnActorFromClass` _placeableactortype (`KismetMathLibrary.MakeTransform` (0.0 0.0 -100000.0)) "AlwaysSpawn" "MultiplyWithRoot" null null))
      (bind _asbp_placable_structure_2 (cast `/Game/Game/Blueprints/Structures/BP_PlacableStructure` _returnvalue_2))
      (set `self.PlaceableActor` _asbp_placable_structure_2)
      (`/Engine/EditorBlueprintResources/StandardMacros.IsValid` _struc_old_3
        (:`Is Valid`
          (set `/Game/Game/Blueprints/Structures/BP_PlacableStructure.Structure Info` (`/Game/Game/Blueprints/Structures/BP_PlacableStructure.Structure Info` _struc_old_3) _placeableactor_2)
          (set `/Game/Game/Blueprints/Structures/BP_PlacableStructure.Info` (`/Game/Game/Blueprints/Structures/BP_PlacableStructure.Info` _struc_old_3) _placeableactor_2))
        (:`Is Not Valid`
          (bind _structure_info_2 (`/Game/Game/Blueprints/Structures/BP_PlacableStructure.Structure Info` _returnvalue_2))
          (set `/Game/Game/Blueprints/Structures/BP_PlacableStructure.Structure Info` _structure_info_2 _placeableactor_2)
          (set `/Game/Game/Blueprints/Structures/BP_PlacableStructure.Info` (`/Game/Game/Blueprints/DataAsset/BP_DataAsset_Structure.Info` _structure_info_2) _placeableactor_2)))
      (`AddComponent|NODE_AddBP_PloppableComponent-0` :`self` _placeableactor_2))))

(fn `ResetBuilding`
  (bind _struc_old (`self.Struc Old`))
  (bind _struc_old_2 (`self.Struc Old`))
  (bind _gridcell (`/Game/Game/Blueprints/Structures/BP_PlacableStructure.GridCell` _struc_old_2))
  (bind _returnvalue (`|SpawnActorFromClass` (`GameplayStatics.GetObjectClass` _struc_old) (`KismetMathLibrary.MakeTransform` (.location (`self.GetTransform` _struc_old)) (.rotation (`self.GetTransform` _struc_old)) (.scale (`self.GetTransform` _struc_old))) "AlwaysSpawn" "MultiplyWithRoot" null null))
  (bind _asbp_placable_structure (cast `/Game/Game/Blueprints/Structures/BP_PlacableStructure` _returnvalue))
  (`/Game/Game/Blueprints/Structures/BP_PlacableStructure.Initialise` _asbp_placable_structure (`/Game/Game/Blueprints/Structures/BP_PlacableStructure.Structure Info` _struc_old_2) (`/Game/Game/Blueprints/Structures/BP_PlacableStructure.Info` _struc_old_2) false)
  (set `/Game/Game/Blueprints/Structures/BP_PlacableStructure.GridCell` _gridcell _asbp_placable_structure)
  (`/Game/Game/Blueprints/Grid/BP_GridCell.SetOccupied` _gridcell (`/Game/Game/Blueprints/Structures/BP_PlacableStructure.BuildingType` _asbp_placable_structure) _returnvalue (`KismetStringLibrary.LeftChop` (`KismetSystemLibrary.GetClassDisplayName` (`GameplayStatics.GetObjectClass` _struc_old)) 2))
  (bind _asbp_road (cast `/Game/Game/Blueprints/Structures/BP_Road` _returnvalue)
    (:`then`
      (bind _returnvalue_2 (`GameplayStatics.GetActorOfClass` "/Game/Game/Blueprints/Road/BP_RoadManager.BP_RoadManager_C"))
      (`/Game/Game/Blueprints/Road/BP_RoadManager.AddRoadTile` _returnvalue_2 _asbp_road))
    (:`CastFailed`
      _))
  (if (`self.Unique`)
    (`self.K2_DestroyActor` (`self.Struc Old`))
    (set `self.Unique` false)
    (`self.OnPlacementInfoUpdated` null)))

(fn `SetPlacementModeEnable`
  (params (IsEnable :type Boolean))
  (bind _placeableactor (`self.PlaceableActor`))
  (if (== (`self.PlacementModeEnable`) IsEnable)
    (return)
    (else
      (bind _output_get (set `self.PlacementModeEnable` IsEnable))
      (if _output_get
        (`self.K2_DestroyActor` _placeableactor)
        (`self.RefreshPlaceableBuilding`)
        (else
          (`/Engine/EditorBlueprintResources/StandardMacros.IsValid` _placeableactor
            (:`Is Valid`
              (`self.K2_DestroyActor` _placeableactor))))))))

(fn `SpawnBuilding`
  (bind _placeableactor (`self.PlaceableActor`))
  (bind _placeableactor_2 (`self.PlaceableActor`))
  (bind _returnvalue (`self.GetComponentByClass` (`self.PlaceableActor`) "/Game/Game/Blueprints/Component/BP_PloppableComponent.BP_PloppableComponent_C"))
  (bind _info_name (break `/Game/Game/Blueprints/DataAsset/S_Info` (`/Game/Game/Blueprints/Structures/BP_PlacableStructure.Info` _placeableactor_2)))
  (`/Engine/EditorBlueprintResources/StandardMacros.IsValid` _returnvalue
    (:`Is Valid`
      (if (`/Game/Game/Blueprints/Component/BP_PloppableComponent.IsPlacementValid` _returnvalue)
        (bind _asbp_player_game_instance (cast `/Game/Game/Saves/BP_PlayerGameInstance` (`GameplayStatics.GetGameInstance`)))
        (bind _stats_money (break `/Game/Game/Blueprints/DataAsset/S_StatsStart` (`/Game/Game/Saves/BP_PlayerGameInstance.Stats` _asbp_player_game_instance)))
        (if (or (`self.Unique`) (>= _stats_money (`.Cost_8_DA7CA1B0407C2DC38A4CFBB7F7445C96` (break `/Game/Game/Blueprints/DataAsset/S_Info` (`/Game/Game/Blueprints/Structures/BP_PlacableStructure.Info` _placeableactor)))))
          (bind _returnvalue_2 (`|SpawnActorFromClass` (`self.PlaceableActorType`) (`KismetMathLibrary.MakeTransform` (- (.location (`self.GetTransform` _placeableactor)) (0.0 0.0 50.0)) (.rotation (`self.GetTransform` _placeableactor)) (.scale (`self.GetTransform` _placeableactor))) "AlwaysSpawn" "MultiplyWithRoot" null null))
          (bind _returnvalue_3 (`GameplayStatics.GetActorOfClass` "/Game/Game/Blueprints/Grid/BP_Grid.BP_Grid_C"))
          (bind _outputcell (`/Game/Game/Blueprints/Grid/BP_Grid.GetClosestGridCell` _returnvalue_3 (`self.K2_GetActorLocation` (`self.PlaceableActor`))))
          (bind _asbp_placable_structure (cast `/Game/Game/Blueprints/Structures/BP_PlacableStructure` _returnvalue_2))
          (set `/Game/Game/Blueprints/Structures/BP_PlacableStructure.GridCell` _outputcell _asbp_placable_structure)
          (`/Game/Game/Blueprints/Structures/BP_PlacableStructure.Initialise` _asbp_placable_structure (`/Game/Game/Blueprints/Structures/BP_PlacableStructure.Structure Info` _placeableactor_2) (`/Game/Game/Blueprints/Structures/BP_PlacableStructure.Info` _placeableactor_2) (`self.Unique`))
          (`/Game/Game/Blueprints/Grid/BP_GridCell.SetOccupied` _outputcell (`/Game/Game/Blueprints/Structures/BP_PlacableStructure.BuildingType` _asbp_placable_structure) _returnvalue_2 _info_name)
          (bind _asbp_road (cast `/Game/Game/Blueprints/Structures/BP_Road` _returnvalue_2)
            (:`then`
              (bind _returnvalue_4 (`GameplayStatics.GetActorOfClass` "/Game/Game/Blueprints/Road/BP_RoadManager.BP_RoadManager_C"))
              (`/Game/Game/Blueprints/Road/BP_RoadManager.AddRoadTile` _returnvalue_4 _asbp_road))
            (:`CastFailed`
              _))
          (if (`self.Unique`)
            (`self.K2_DestroyActor` (`self.Struc Old`))
            (set `self.Unique` false)
            (`self.OnPlacementInfoUpdated` null))
          (else
            (bind _asbp_uihud (cast `/Game/Game/Blueprints/HUD/BP_UIHUD` (`self.GetHUD` (`GameplayStatics.GetPlayerController` 0))))
            (`/Game/Game/UI/WB_MainGame.Error` (`/Game/Game/Blueprints/HUD/BP_UIHUD.MainGame` _asbp_uihud) "You don't have enough money!")))
        (else
          (bind _asbp_uihud_2 (cast `/Game/Game/Blueprints/HUD/BP_UIHUD` (`self.GetHUD` (`GameplayStatics.GetPlayerController` 0))))
          (`/Game/Game/UI/WB_MainGame.Error` (`/Game/Game/Blueprints/HUD/BP_UIHUD.MainGame` _asbp_uihud_2) "The placement is invalid!"))))))

(fn `UpdatePlacement`
  (bind (_worldlocation _worlddirection) (`self.DeprojectMousePositionToWorld`))
  (bind _outhit (`KismetSystemLibrary.LineTraceSingle` _worldlocation (+ _worlddirection (* _worlddirection 1000000.0)) "TraceTypeQuery3"))
  (bind (_bblockinghit _binitialoverlap _time _distance _location) (`GameplayStatics.BreakHitResult` _outhit))
  (if _bblockinghit
    (bind _returnvalue (`GameplayStatics.GetActorOfClass` "/Game/Game/Blueprints/Grid/BP_Grid.BP_Grid_C"))
    (bind _outputvector (`/Game/Game/Blueprints/Grid/BP_Grid.GetClosestGridPosition` _returnvalue _location))
    (`self.K2_SetActorLocation` (`self.PlaceableActor`) (+ _outputvector (0.0 0.0 100.0)) false false)))

(fn `UserConstructionScript`)