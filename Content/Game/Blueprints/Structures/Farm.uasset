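; Farm is a structure Blueprint that makes its Cube component respond to mouse clicks and hovering.
; On BeginPlay it enables click and mouse-over events on the first player controller.
; The Cube's click event passes the actor to Click, while cursor enter and exit pass the Cube to MouseStartOver and MouseEndOver.
; The graph contains no farm-specific logic, and its overlap and Tick events are disabled.
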(event `self.ReceiveBeginPlay`
  (bind _returnvalue (`GameplayStatics.GetPlayerController` 0))
  (set `PlayerController.bEnableClickEvents` true _returnvalue)
  (set `PlayerController.bEnableMouseOverEvents` true _returnvalue)
  (`parent.ReceiveBeginPlay`))

(event `self.Cube.OnClicked`
  (params (TouchedComponent :type "PrimitiveComponent Object Reference") (ButtonPressed :type "Key Structure"))
  (`self.Click` self))

(event `self.Cube.OnBeginCursorOver`
  (params (TouchedComponent :type "PrimitiveComponent Object Reference"))
  (`self.Mouse Start Over` (`self.Cube`)))

(event `self.Cube.OnEndCursorOver`
  (params (TouchedComponent :type "PrimitiveComponent Object Reference"))
  (`self.Mouse End Over` (`self.Cube`)))

(fn `UserConstructionScript`
  (`parent.UserConstructionScript`))