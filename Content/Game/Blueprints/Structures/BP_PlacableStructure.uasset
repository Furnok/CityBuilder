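; BP_PlacableStructure is a placed grid structure in a building game that can be selected or demolished.
; Outside placement mode, hover toggles custom depth and a camera-facing level label, while click opens the structure UI or, in destroy mode, demolishes it.
; One building type reacts only in destroy mode.
; Initialise charges non-unique structures and updates population cap and HUD; demolition frees the grid cell and resets BP_RoadManager's roads.
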(event `Destroy`
  (`/Game/Game/Blueprints/Grid/BP_GridCell.SetUnOccupied` (`self.GridCell`))
  (`self.SetActorHiddenInGame` (stale `Click` Actor) true)
  (bind _returnvalue (`GameplayStatics.GetActorOfClass` "/Game/Game/Blueprints/Road/BP_RoadManager.BP_RoadManager_C"))
  (`/Game/Game/Blueprints/Road/BP_RoadManager.ResetRoad` _returnvalue))

(event `Click`
  (params (Actor :type "Actor Object Reference"))
  (bind _asbp_player_controller (cast `/Game/Game/Blueprints/Controller/BP_PlayerController` (`GameplayStatics.GetPlayerController` 0)))
  (if (`/Game/Game/Blueprints/Controller/BP_PlayerController.PlacementModeEnable` _asbp_player_controller)
    _
    (elif (`/Game/Game/Blueprints/Controller/BP_PlayerController.DestroyModeEnable` _asbp_player_controller)
      (`self.K2_DestroyActor` Actor :!label _label)
      (`/Game/Game/Blueprints/Grid/BP_GridCell.SetUnOccupied` (`self.GridCell`))
      (`/Engine/EditorBlueprintResources/StandardMacros.IsValid` Actor
        (:`Is Valid`
          (`self.SetActorHiddenInGame` Actor true))
        (:`Is Not Valid`
          _))
      (bind _returnvalue (`GameplayStatics.GetActorOfClass` "/Game/Game/Blueprints/Road/BP_RoadManager.BP_RoadManager_C"))
      (`/Game/Game/Blueprints/Road/BP_RoadManager.ResetRoad` _returnvalue)
      (elif (`|EnumInequality` (`self.BuildingType`) "NewEnumerator2")
        (bind _asbp_uihud (cast `/Game/Game/Blueprints/HUD/BP_UIHUD` (`PlayerController.GetHUD` (`GameplayStatics.GetPlayerController` 0))))
        (`/Game/Game/Blueprints/HUD/BP_UIHUD.Structure UI` _asbp_uihud false self)
        (bind _asbp_uihud_2 (cast `/Game/Game/Blueprints/HUD/BP_UIHUD` (`PlayerController.GetHUD` (`GameplayStatics.GetPlayerController` 0))))
        (`/Game/Game/UI/WB_MainGame.Remove` (`/Game/Game/Blueprints/HUD/BP_UIHUD.MainGame` _asbp_uihud_2))))))

(event `self.ReceiveTick`
  (params (DeltaSeconds :type "Float (single-precision)"))
  (if (`SceneComponent.IsVisible` (`self.TextRender`))
    (`SceneComponent.K2_SetWorldRotation` (`self.TextRender`) (`KismetMathLibrary.MakeRotator` 0.0 0.0 (.yaw (`KismetMathLibrary.FindLookAtRotation` (`self.K2_GetActorLocation`) (`PlayerCameraManager.GetCameraLocation` (`GameplayStatics.GetPlayerCameraManager` 0))))) false false)))

(event `DestroyAll`
  (goto _label))

(event `Mouse Start Over`
  (params (Actor :type "StaticMeshComponent Object Reference"))
  (bind _asbp_player_controller (cast `/Game/Game/Blueprints/Controller/BP_PlayerController` (`GameplayStatics.GetPlayerController` 0)))
  (if (`/Game/Game/Blueprints/Controller/BP_PlayerController.PlacementModeEnable` _asbp_player_controller)
    _
    (elif (`|EnumEquality` (`self.BuildingType`) "NewEnumerator2")
      (bind _asbp_player_controller_2 (cast `/Game/Game/Blueprints/Controller/BP_PlayerController` (`GameplayStatics.GetPlayerController` 0)))
      (if (`/Game/Game/Blueprints/Controller/BP_PlayerController.DestroyModeEnable` _asbp_player_controller_2)
        (`PrimitiveComponent.SetRenderCustomDepth` Actor true))
      (else
        (`PrimitiveComponent.SetRenderCustomDepth` Actor true)
        (`SceneComponent.SetVisibility` (`self.TextRender`) true false)
        (`TextRenderComponent.K2_SetText` (`self.TextRender`) (`KismetTextLibrary.Conv_StringToText` (`KismetStringLibrary.Concat_StrStr` (`/Game/Game/Blueprints/Grid/BP_GridCell.Name` (`self.GridCell`)) " Level " (`KismetTextLibrary.Conv_TextToString` (`KismetTextLibrary.Conv_IntToText` (`.Level_6_915C2CEE448C2650F67EF7925E09986A` (break `/Game/Game/Blueprints/DataAsset/S_Info` (`self.Info`))))))) :!label _label_2)))))

(event `Update Level`
  (goto _label_2))

(event `Mouse End Over`
  (params (Actor :type "StaticMeshComponent Object Reference"))
  (bind _asbp_player_controller (cast `/Game/Game/Blueprints/Controller/BP_PlayerController` (`GameplayStatics.GetPlayerController` 0)))
  (if (`/Game/Game/Blueprints/Controller/BP_PlayerController.PlacementModeEnable` _asbp_player_controller)
    _
    (elif (`|EnumEquality` (`self.BuildingType`) "NewEnumerator2")
      (bind _asbp_player_controller_2 (cast `/Game/Game/Blueprints/Controller/BP_PlayerController` (`GameplayStatics.GetPlayerController` 0)))
      (if (`/Game/Game/Blueprints/Controller/BP_PlayerController.DestroyModeEnable` _asbp_player_controller_2)
        (`PrimitiveComponent.SetRenderCustomDepth` Actor false))
      (else
        (`PrimitiveComponent.SetRenderCustomDepth` Actor false)
        (`SceneComponent.SetVisibility` (`self.TextRender`) false false)))))

(fn `Initialise`
  (params (Structure :type "/Game/Game/Blueprints/DataAsset/BP_DataAsset_Structure Object Reference") (Info :type "/Game/Game/Blueprints/DataAsset/S_Info Structure") (Unique :type Boolean))
  (bind (_info_name _info_description _info_level _info_levelmax _info_population _info_radius _info_satisfaction _info_money _info_cost) (break `/Game/Game/Blueprints/DataAsset/S_Info` (`self.Info`)))
  (set `self.Structure Info` Structure)
  (set `self.Info` Info)
  (if (not Unique)
    (bind _asbp_player_game_instance (cast `/Game/Game/Saves/BP_PlayerGameInstance` (`GameplayStatics.GetGameInstance`)))
    (if (> _info_population 0)
      (bind (_stats_money _stats_satisfaction _stats_population _stats_populationmax) (break `/Game/Game/Blueprints/DataAsset/S_StatsStart` (`/Game/Game/Saves/BP_PlayerGameInstance.Stats` _asbp_player_game_instance)))
      (bind _returnvalue (- _stats_money _info_cost))
      (set `/Game/Game/Saves/BP_PlayerGameInstance.Stats` (make `/Game/Game/Blueprints/DataAsset/S_StatsStart` _returnvalue _stats_satisfaction _stats_population (+ _stats_populationmax 1)) _asbp_player_game_instance)
      (else
        (set `/Game/Game/Saves/BP_PlayerGameInstance.Stats` (make `/Game/Game/Blueprints/DataAsset/S_StatsStart` _returnvalue _stats_satisfaction _stats_population _stats_populationmax) _asbp_player_game_instance)))
    (bind _asbp_uihud (cast `/Game/Game/Blueprints/HUD/BP_UIHUD` (`PlayerController.GetHUD` (`GameplayStatics.GetPlayerController` 0))))
    (`/Game/Game/UI/WB_MainGame.Initialisation UI` (`/Game/Game/Blueprints/HUD/BP_UIHUD.MainGame` _asbp_uihud))))

(fn `UserConstructionScript`)