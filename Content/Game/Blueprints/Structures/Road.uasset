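; Road structure for a tile grid that adjusts its four side pathway components to match neighbouring tiles.
; On BeginPlay it sets its building type, apparently the road value of the enum.
; Whenever OnNewTileAdded fires, it checks each cardinal neighbour cell, hiding that side's pathway if the occupying type matches and showing it otherwise.
; Sides without a valid neighbour cell are left unchanged.
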(event `self.ReceiveBeginPlay`
  (`parent.ReceiveBeginPlay`)
  (set `self.BuildingType` "NewEnumerator2"))

(event `OnNewTileAdded`
  (bind _gridcell (`self.GridCell`))
  (`self.UpdateSideOfRoadTile` (`/Game/Game/Blueprints/Grid/GridCell.NeighbourNorth` _gridcell) (`self.PathwayNorth`))
  (`self.UpdateSideOfRoadTile` (`/Game/Game/Blueprints/Grid/GridCell.NeighbourSouth` _gridcell) (`self.PathwaySouth`))
  (`self.UpdateSideOfRoadTile` (`/Game/Game/Blueprints/Grid/GridCell.NeighbourWest` _gridcell) (`self.PathwayWeast`))
  (`self.UpdateSideOfRoadTile` (`/Game/Game/Blueprints/Grid/GridCell.NeighbourEast` _gridcell) (`self.PathwayEast`)))

(fn `UpdateSideOfRoadTile`
  (params (`Grid Cell` :type "/Game/Game/Blueprints/Grid/GridCell Object Reference") (Pathway :type "StaticMeshComponent Object Reference"))
  (`/Engine/EditorBlueprintResources/StandardMacros.IsValid` `Grid Cell`
    (:`Is Valid`
      (if (`|EnumEquality` (`/Game/Game/Blueprints/Grid/GridCell.OccupingType` `Grid Cell`) "NewEnumerator2")
        (`SceneComponent.SetVisibility` Pathway false false)
        (else
          (`SceneComponent.SetVisibility` Pathway true false))))))

(fn `UserConstructionScript`
  (`parent.UserConstructionScript`))