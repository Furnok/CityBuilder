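; BP_Road is the road structure for a grid-based building game, setting its building type and structure info on BeginPlay.
; When a new tile is added, it checks its four grid neighbours and hides the pathway piece on sides whose occupying type matches the road enumerator, showing it otherwise.
; Invalid neighbour cells leave their side unchanged.
; Its cube forwards click and hover events, with mouse events enabled on the player controller.
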(event `self.ReceiveBeginPlay`
  (bind _returnvalue (`GameplayStatics.GetPlayerController` 0))
  (set `PlayerController.bEnableClickEvents` true _returnvalue)
  (set `PlayerController.bEnableMouseOverEvents` true _returnvalue)
  (`parent.ReceiveBeginPlay`)
  (set `self.BuildingType` "NewEnumerator2")
  (set `self.Structure Info` (`self.Structure Info_0`)))

(event `OnNewTileAdded`
  (bind _gridcell (`self.GridCell`))
  (`self.UpdateSideOfRoadTile` (`/Game/Game/Blueprints/Grid/BP_GridCell.NeighbourNorth` _gridcell) (`self.PathwayNorth`))
  (`self.UpdateSideOfRoadTile` (`/Game/Game/Blueprints/Grid/BP_GridCell.NeighbourSouth` _gridcell) (`self.PathwaySouth`))
  (`self.UpdateSideOfRoadTile` (`/Game/Game/Blueprints/Grid/BP_GridCell.NeighbourWest` _gridcell) (`self.PathwayWeast`))
  (`self.UpdateSideOfRoadTile` (`/Game/Game/Blueprints/Grid/BP_GridCell.NeighbourEast` _gridcell) (`self.PathwayEast`)))

(event `self.Cube.OnClicked`
  (params (TouchedComponent :type "PrimitiveComponent Object Reference") (ButtonPressed :type "Key Structure"))
  (`self.Click` self))

(event `self.Cube.OnBeginCursorOver`
  (params (TouchedComponent :type "PrimitiveComponent Object Reference"))
  (`self.Mouse Start Over` (`self.Cube`)))

(event `self.Cube.OnEndCursorOver`
  (params (TouchedComponent :type "PrimitiveComponent Object Reference"))
  (`self.Mouse End Over` (`self.Cube`)))

(fn `UpdateSideOfRoadTile`
  (params (`Grid Cell` :type "/Game/Game/Blueprints/Grid/BP_GridCell Object Reference") (Pathway :type "StaticMeshComponent Object Reference"))
  (`/Engine/EditorBlueprintResources/StandardMacros.IsValid` `Grid Cell`
    (:`Is Valid`
      (if (`|EnumEquality` (`/Game/Game/Blueprints/Grid/BP_GridCell.OccupingType` `Grid Cell`) "NewEnumerator2")
        (`SceneComponent.SetVisibility` Pathway false false)
        (else
          (`SceneComponent.SetVisibility` Pathway true false))))))

(fn `UserConstructionScript`
  (`parent.UserConstructionScript`))