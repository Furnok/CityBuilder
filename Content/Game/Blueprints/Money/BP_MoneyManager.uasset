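; BP_MoneyManager runs the colony economy: income, population growth and satisfaction decay.
; BeginPlay starts three self-rescheduling Delay loops that update the Stats struct in BP_PlayerGameInstance and refresh the HUD.
; Collect sums farm money from the BP_Grid cells every DurationC seconds, and PopulationCome adds residents at random intervals.
; LoseSatisfaction periodically lowers clamped satisfaction while population exceeds its maximum.
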(event `self.ReceiveBeginPlay`
  (`|ExecutionSequence`
    (:`then_0`
      (`KismetSystemLibrary.Delay` (`self.DurationC`))
      (`self.Collect`))
    (:`then_1`
      (`KismetSystemLibrary.Delay` (`KismetMathLibrary.Conv_IntToDouble` (`KismetMathLibrary.RandomIntegerInRange` 5 15)))
      (`self.Population Come`))
    (:`then_2`
      (`KismetSystemLibrary.Delay` 3.0)
      (`self.LoseSatisfaction`))))

(event `Collect`
  (set `self.Add` 0)
  (bind _returnvalue (`GameplayStatics.GetActorOfClass` "/Game/Game/Blueprints/Grid/BP_Grid.BP_Grid_C"))
  (for _array_element (`/Game/Game/Blueprints/Grid/BP_Grid.GridArray` _returnvalue)
    (bind _asbp_farm (cast `/Game/Game/Blueprints/Structures/BP_Farm` (`/Game/Game/Blueprints/Grid/BP_GridCell.OccupingActor` _array_element)))
    (bind (_info_name _info_description _info_level _info_levelmax _info_population _info_radius _info_satisfaction _info_money) (break `/Game/Game/Blueprints/DataAsset/S_Info` (`/Game/Game/Blueprints/Structures/BP_PlacableStructure.Info` _asbp_farm)))
    (set `self.Add` (+ (`self.Add`) _info_money)))
  (bind _asbp_player_game_instance (cast `/Game/Game/Saves/BP_PlayerGameInstance` (`GameplayStatics.GetGameInstance`)))
  (bind (_stats_money _stats_satisfaction _stats_population _stats_populationmax) (break `/Game/Game/Blueprints/DataAsset/S_StatsStart` (`/Game/Game/Saves/BP_PlayerGameInstance.Stats` _asbp_player_game_instance)))
  (set `/Game/Game/Saves/BP_PlayerGameInstance.Stats` (make `/Game/Game/Blueprints/DataAsset/S_StatsStart` (+ _stats_money (`self.Add`)) _stats_satisfaction _stats_population _stats_populationmax) _asbp_player_game_instance)
  (bind _asbp_uihud (cast `/Game/Game/Blueprints/HUD/BP_UIHUD` (`PlayerController.GetHUD` (`GameplayStatics.GetPlayerController` 0))))
  (`/Game/Game/UI/WB_MainGame.Initialisation UI` (`/Game/Game/Blueprints/HUD/BP_UIHUD.MainGame` _asbp_uihud))
  (`KismetSystemLibrary.Delay` (`self.DurationC`))
  (`self.Collect`))

(event `Population Come`
  (bind _asbp_player_game_instance (cast `/Game/Game/Saves/BP_PlayerGameInstance` (`GameplayStatics.GetGameInstance`)))
  (bind (_stats_money _stats_satisfaction _stats_population _stats_populationmax) (break `/Game/Game/Blueprints/DataAsset/S_StatsStart` (`/Game/Game/Saves/BP_PlayerGameInstance.Stats` _asbp_player_game_instance)))
  (set `/Game/Game/Saves/BP_PlayerGameInstance.Stats` (make `/Game/Game/Blueprints/DataAsset/S_StatsStart` _stats_money _stats_satisfaction (+ _stats_population (`KismetMathLibrary.RandomIntegerInRange` 1 3)) _stats_populationmax) _asbp_player_game_instance)
  (bind _asbp_uihud (cast `/Game/Game/Blueprints/HUD/BP_UIHUD` (`PlayerController.GetHUD` (`GameplayStatics.GetPlayerController` 0))))
  (`/Game/Game/UI/WB_MainGame.Initialisation UI` (`/Game/Game/Blueprints/HUD/BP_UIHUD.MainGame` _asbp_uihud))
  (`KismetSystemLibrary.Delay` (`KismetMathLibrary.Conv_IntToDouble` (`KismetMathLibrary.RandomIntegerInRange` 5 15)))
  (`self.Population Come`))

(event `LoseSatisfaction`
  (bind _asbp_player_game_instance (cast `/Game/Game/Saves/BP_PlayerGameInstance` (`GameplayStatics.GetGameInstance`)))
  (bind (_stats_money _stats_satisfaction _stats_population _stats_populationmax) (break `/Game/Game/Blueprints/DataAsset/S_StatsStart` (`/Game/Game/Saves/BP_PlayerGameInstance.Stats` _asbp_player_game_instance)))
  (if (> _stats_population _stats_populationmax)
    (set `/Game/Game/Saves/BP_PlayerGameInstance.Stats` (make `/Game/Game/Blueprints/DataAsset/S_StatsStart` _stats_money (`KismetMathLibrary.Clamp` (- _stats_satisfaction 1) 0 100) _stats_population _stats_populationmax) _asbp_player_game_instance)
    (bind _asbp_uihud (cast `/Game/Game/Blueprints/HUD/BP_UIHUD` (`PlayerController.GetHUD` (`GameplayStatics.GetPlayerController` 0))))
    (`/Game/Game/UI/WB_MainGame.Initialisation UI` (`/Game/Game/Blueprints/HUD/BP_UIHUD.MainGame` _asbp_uihud))
    (`KismetSystemLibrary.Delay` 3.0)
    (`self.LoseSatisfaction`)
    (else
      (`KismetSystemLibrary.Delay` 3.0)
      (`self.LoseSatisfaction`))))

(fn `UserConstructionScript`)