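; Placement preview component that shows whether its owning actor can be placed on the grid at its current location.
; Every tick it finds the closest BP_Grid cell and treats it as valid if unoccupied.
; For road-type BP_PlacableStructure owners, RoadPlacableCheck also rejects cells that would complete a 2x2 road block in any diagonal direction.
; The result swaps the first material slot on all owner static meshes between valid and invalid materials.
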(event `self.ReceiveBeginPlay`
  (`self.UpdateState`))

(event `self.ReceiveTick`
  (params (DeltaSeconds :type "Float (single-precision)"))
  (`self.UpdateState`))

(fn `RoadPlacableCheck`
  (params (GridCell :type "/Game/Game/Blueprints/Grid/BP_GridCell Object Reference"))
  (bind _neighboureast (`/Game/Game/Blueprints/Grid/BP_GridCell.NeighbourEast` GridCell))
  (bind _neighbournorth (`/Game/Game/Blueprints/Grid/BP_GridCell.NeighbourNorth` GridCell))
  (bind _neighboursouth (`/Game/Game/Blueprints/Grid/BP_GridCell.NeighbourSouth` GridCell))
  (bind _neighbourwest (`/Game/Game/Blueprints/Grid/BP_GridCell.NeighbourWest` GridCell))
  (bind _returnvalue (`KismetSystemLibrary.IsValid` _neighboursouth))
  (bind _returnvalue_2 (`KismetSystemLibrary.IsValid` _neighbournorth))
  (bind _returnvalue_3 (`KismetSystemLibrary.IsValid` _neighbourwest))
  (bind _returnvalue_4 (`KismetSystemLibrary.IsValid` _neighboureast))
  (bind _neighbourwest_2 (`/Game/Game/Blueprints/Grid/BP_GridCell.NeighbourWest` _neighboursouth))
  (bind _neighboureast_2 (`/Game/Game/Blueprints/Grid/BP_GridCell.NeighbourEast` _neighboursouth))
  (bind _neighbourwest_3 (`/Game/Game/Blueprints/Grid/BP_GridCell.NeighbourWest` _neighbournorth))
  (bind _neighboureast_3 (`/Game/Game/Blueprints/Grid/BP_GridCell.NeighbourEast` _neighbournorth))
  (bind _returnvalue_5 (`|EnumEquality` (`/Game/Game/Blueprints/Grid/BP_GridCell.OccupingType` _neighboureast) "NewEnumerator2"))
  (bind _returnvalue_6 (`|EnumEquality` (`/Game/Game/Blueprints/Grid/BP_GridCell.OccupingType` _neighbournorth) "NewEnumerator2"))
  (bind _returnvalue_7 (`|EnumEquality` (`/Game/Game/Blueprints/Grid/BP_GridCell.OccupingType` _neighboursouth) "NewEnumerator2"))
  (bind _returnvalue_8 (`|EnumEquality` (`/Game/Game/Blueprints/Grid/BP_GridCell.OccupingType` _neighbourwest) "NewEnumerator2"))
  (bind _asbp_placable_structure (cast `/Game/Game/Blueprints/Structures/BP_PlacableStructure` (`self.GetOwner`))
    (:`then`
      (if (`|EnumEquality` (`/Game/Game/Blueprints/Structures/BP_PlacableStructure.BuildingType` _asbp_placable_structure) "NewEnumerator2")
        (if (and _returnvalue_2 _returnvalue_3)
          (if (and _returnvalue_6 _returnvalue_8)
            (`/Engine/EditorBlueprintResources/StandardMacros.IsValid` _neighbourwest_3
              (:`Is Valid`
                (if (`|EnumEquality` (`/Game/Game/Blueprints/Grid/BP_GridCell.OccupingType` _neighbourwest_3) "NewEnumerator2")
                  (set `self.IsPlacementValid` false)
                  (return)
                  (else
                    _)))
              (:`Is Not Valid`
                _))))
        (if (and _returnvalue_2 _returnvalue_4)
          (if (and _returnvalue_6 _returnvalue_5)
            (`/Engine/EditorBlueprintResources/StandardMacros.IsValid` _neighboureast_3
              (:`Is Valid`
                (if (`|EnumEquality` (`/Game/Game/Blueprints/Grid/BP_GridCell.OccupingType` _neighboureast_3) "NewEnumerator2")
                  (set `self.IsPlacementValid` false)
                  (return)
                  (else
                    _)))
              (:`Is Not Valid`
                _))))
        (if (and _returnvalue _returnvalue_3)
          (if (and _returnvalue_7 _returnvalue_8)
            (`/Engine/EditorBlueprintResources/StandardMacros.IsValid` _neighbourwest_2
              (:`Is Valid`
                (if (`|EnumEquality` (`/Game/Game/Blueprints/Grid/BP_GridCell.OccupingType` _neighbourwest_2) "NewEnumerator2")
                  (set `self.IsPlacementValid` false)
                  (return)
                  (else
                    _)))
              (:`Is Not Valid`
                _))))
        (if (and _returnvalue _returnvalue_4)
          (if (and _returnvalue_7 _returnvalue_5)
            (`/Engine/EditorBlueprintResources/StandardMacros.IsValid` _neighboureast_2
              (:`Is Valid`
                (if (`|EnumEquality` (`/Game/Game/Blueprints/Grid/BP_GridCell.OccupingType` _neighboureast_2) "NewEnumerator2")
                  (set `self.IsPlacementValid` false)
                  (return))))))
        (else
          (return))))
    (:`CastFailed`
      (return))))

(fn `UpdateState`
  (bind _returnvalue (`GameplayStatics.GetActorOfClass` "/Game/Game/Blueprints/Grid/BP_Grid.BP_Grid_C"))
  (bind _outputcell (`/Game/Game/Blueprints/Grid/BP_Grid.GetClosestGridCell` _returnvalue (`Actor.K2_GetActorLocation` (`self.GetOwner`))))
  (bind _output_get (set `self.IsPlacementValid` (not (`/Game/Game/Blueprints/Grid/BP_GridCell.IsOccupied` _outputcell))))
  (`self.RoadPlacableCheck` _outputcell)
  (for _array_element (`Actor.K2_GetComponentsByClass` (`self.GetOwner`) "/Script/Engine.StaticMeshComponent")
    (if _output_get
      (`PrimitiveComponent.SetMaterial` _array_element 0 (`self.PloppableMaterial`))
      (else
        (`PrimitiveComponent.SetMaterial` _array_element 0 (`self.InvalidPloppableMaterial`))))))