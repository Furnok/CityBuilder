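; Placement-preview component for grid building that shows whether its owner actor can be placed at its current location.
; On begin play and each overlap begin or end, it finds the closest Grid cell, marks placement valid if unoccupied, and applies the valid or invalid material to the owner's static meshes.
; A road check meant to reject 2x2 road blocks through diagonal neighbour tests exists but is disconnected.
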(event `self.ReceiveBeginPlay`
  (bind _returnvalue (`self.GetOwner`))
  (add `Actor.OnActorBeginOverlap` _returnvalue (delegate `State`))
  (add `Actor.OnActorEndOverlap` _returnvalue (delegate `State`))
  (`self.UpdateState`))

(event `State`
  (params (OverlappedActor :type "Actor Object Reference") (OtherActor :type "Actor Object Reference"))
  (`self.UpdateState`))

(fn `RoadPlacableCheck`
  (params (GridCell :type "/Game/Game/Blueprints/Grid/GridCell Object Reference"))
  (bind _neighboureast (`/Game/Game/Blueprints/Grid/GridCell.NeighbourEast` GridCell))
  (bind _neighbournorth (`/Game/Game/Blueprints/Grid/GridCell.NeighbourNorth` GridCell))
  (bind _neighboursouth (`/Game/Game/Blueprints/Grid/GridCell.NeighbourSouth` GridCell))
  (bind _neighbourwest (`/Game/Game/Blueprints/Grid/GridCell.NeighbourWest` GridCell))
  (bind _returnvalue (`KismetSystemLibrary.IsValid` _neighbournorth))
  (bind _neighbourwest_2 (`/Game/Game/Blueprints/Grid/GridCell.NeighbourWest` _neighboursouth))
  (bind _neighboureast_2 (`/Game/Game/Blueprints/Grid/GridCell.NeighbourEast` _neighboursouth))
  (bind _neighbourwest_3 (`/Game/Game/Blueprints/Grid/GridCell.NeighbourWest` _neighbournorth))
  (bind _neighboureast_3 (`/Game/Game/Blueprints/Grid/GridCell.NeighbourEast` _neighbournorth))
  (bind _returnvalue_2 (`|EnumEquality` (`/Game/Game/Blueprints/Grid/GridCell.OccupingType` _neighboureast) "NewEnumerator2"))
  (bind _returnvalue_3 (`|EnumEquality` (`/Game/Game/Blueprints/Grid/GridCell.OccupingType` _neighbournorth) "NewEnumerator2"))
  (bind _returnvalue_4 (`|EnumEquality` (`/Game/Game/Blueprints/Grid/GridCell.OccupingType` _neighboursouth) "NewEnumerator2"))
  (bind _returnvalue_5 (`|EnumEquality` (`/Game/Game/Blueprints/Grid/GridCell.OccupingType` _neighbourwest) "NewEnumerator2"))
  (bind _asplacable_structure (cast `/Game/Game/Blueprints/Structures/PlacableStructure` (`self.GetOwner`))
    (:`then`
      (if (`|EnumEquality` (`/Game/Game/Blueprints/Structures/PlacableStructure.BuildingType` _asplacable_structure) "NewEnumerator2")
        (if (and _returnvalue (`KismetSystemLibrary.IsValid` _neighbourwest))
          (if (and _returnvalue_3 _returnvalue_5)
            (`/Engine/EditorBlueprintResources/StandardMacros.IsValid` _neighbourwest_3
              (:`Is Valid`
                (if (`|EnumEquality` (`/Game/Game/Blueprints/Grid/GridCell.OccupingType` _neighbourwest_3) "NewEnumerator2")
                  (set `self.IsPlacementValid` false)
                  (return)
                  (else
                    _)))
              (:`Is Not Valid`
                _))))
        (if (and _returnvalue (`KismetSystemLibrary.IsValid` _neighboureast))
          (if (and _returnvalue_3 _returnvalue_2)
            (`/Engine/EditorBlueprintResources/StandardMacros.IsValid` _neighboureast_3
              (:`Is Valid`
                (if (`|EnumEquality` (`/Game/Game/Blueprints/Grid/GridCell.OccupingType` _neighboureast_3) "NewEnumerator2")
                  (set `self.IsPlacementValid` false)
                  (return)
                  (else
                    _)))
              (:`Is Not Valid`
                _))))
        (if (and _returnvalue_4 _returnvalue_5)
          (`/Engine/EditorBlueprintResources/StandardMacros.IsValid` _neighbourwest_2
            (:`Is Valid`
              (if (`|EnumEquality` (`/Game/Game/Blueprints/Grid/GridCell.OccupingType` _neighbourwest_2) "NewEnumerator2")
                (set `self.IsPlacementValid` false)
                (return)
                (else
                  _)))
            (:`Is Not Valid`
              _)))
        (if (and _returnvalue_4 _returnvalue_2)
          (`/Engine/EditorBlueprintResources/StandardMacros.IsValid` _neighboureast_2
            (:`Is Valid`
              (if (`|EnumEquality` (`/Game/Game/Blueprints/Grid/GridCell.OccupingType` _neighboureast_2) "NewEnumerator2")
                (set `self.IsPlacementValid` false)
                (return)))))
        (else
          (return))))
    (:`CastFailed`
      (return))))

(fn `UpdateState`
  (bind _returnvalue (`GameplayStatics.GetActorOfClass` "/Game/Game/Blueprints/Grid/Grid.Grid_C"))
  (bind _outputcell (`/Game/Game/Blueprints/Grid/Grid.GetClosestGridCell` _returnvalue (`Actor.K2_GetActorLocation` (`self.GetOwner`))))
  (bind _output_get (set `self.IsPlacementValid` (not (`/Game/Game/Blueprints/Grid/GridCell.IsOccupied` _outputcell))))
  (for _array_element (`Actor.K2_GetComponentsByClass` (`self.GetOwner`) "/Script/Engine.StaticMeshComponent")
    (if _output_get
      (`PrimitiveComponent.SetMaterial` _array_element 0 (`self.PloppableMaterial`))
      (else
        (`PrimitiveComponent.SetMaterial` _array_element 0 (`self.InvalidPloppableMaterial`))))))