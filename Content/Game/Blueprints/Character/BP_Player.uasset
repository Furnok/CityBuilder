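; BP_Player is the player-controlled camera, with Enhanced Input actions for orbiting, panning and zooming on a spring arm.
; Rotate adds controller yaw, and Zoom changes the arm length within clamped limits.
; Move applies a swept local offset scaled by arm length, so panning speeds up when zoomed out.
; That offset multiplies world-space forward and right vectors per axis, so its magnitude varies with yaw.
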(event `EnhancedInput|/Game/Game/Inputs/IA_Rotate`
  (params (ActionValue :type "Float (double-precision)") (ElapsedSeconds :type "Float (double-precision)") (TriggeredSeconds :type "Float (double-precision)") (InputAction :type "InputAction Object Reference" :default "/Game/Game/Inputs/IA_Rotate.IA_Rotate"))
  ;[0.016 0.016 0.016] Rotate
  (:`Triggered`
    (`self.AddControllerYawInput` (* ActionValue (`self.OrbitSpeed`)))))

(event `EnhancedInput|/Game/Game/Inputs/IA_Move`
  (params (ActionValue :type "Vector2D Structure") (ElapsedSeconds :type "Float (double-precision)") (TriggeredSeconds :type "Float (double-precision)") (InputAction :type "InputAction Object Reference" :default "/Game/Game/Inputs/IA_Move.IA_Move"))
  (bind _returnvalue (* (`self.InitialCameraSpeed`) (`SpringArmComponent.TargetArmLength` (`self.SpringArm`))))
  ;[0.016 0.016 0.016] Movement
  (:`Triggered`
    (`self.K2_AddActorLocalOffset` (+ (* (`self.GetActorRightVector`) (`KismetMathLibrary.MakeVector` 0.0 (* ActionValue_X _returnvalue))) (* (`self.GetActorForwardVector`) (`KismetMathLibrary.MakeVector` (* ActionValue_Y _returnvalue)))) true)))

(event `EnhancedInput|/Game/Game/Inputs/IA_Zoom`
  (params (ActionValue :type "Float (double-precision)") (ElapsedSeconds :type "Float (double-precision)") (TriggeredSeconds :type "Float (double-precision)") (InputAction :type "InputAction Object Reference" :default "/Game/Game/Inputs/IA_Zoom.IA_Zoom"))
  (bind _springarm (`self.SpringArm`))
  ;[0.016 0.016 0.016] Zoom
  (:`Triggered`
    (set `SpringArmComponent.TargetArmLength` (`KismetMathLibrary.FClamp` (+ (* ActionValue (`self.ZoomSpeed`)) (`SpringArmComponent.TargetArmLength` _springarm)) (`self.ZoomInMax`) (`self.ZoomOutMax`)) _springarm)))

(fn `UserConstructionScript`)