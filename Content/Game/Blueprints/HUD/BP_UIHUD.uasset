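; BP_UIHUD is the UI manager that creates and removes the game's viewport widgets.
; On BeginPlay it shows WB_MainGame and sets Game and UI input focused on it.
; StructureUI removes or shows a WB_Structure panel initialised with a structure, replacing any open panel after a short delay.
; Load and Removes show and clear a WB_Load overlay, created with its Save flag on.
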(event `self.ReceiveBeginPlay`
  (bind _returnvalue (`|CreateWidget` "/Game/Game/UI/WB_MainGame.WB_MainGame_C"))
  (bind _output_get (set `self.MainGame` _returnvalue))
  (`UserWidget.AddToViewport` _output_get 0)
  (`WidgetBlueprintLibrary.SetInputMode_GameAndUIEx` (`GameplayStatics.GetPlayerController` 0) _returnvalue))

(event `Structure UI`
  (params (Del :type Boolean) (Structure :type "/Game/Game/Blueprints/Structures/BP_PlacableStructure Object Reference"))
  (if Del
    (`/Engine/EditorBlueprintResources/StandardMacros.IsValid` (`self.Structure`)
      (:`Is Valid`
        (`Widget.RemoveFromParent` (`self.Structure`))
        (set `self.Structure` null)))
    (else
      (`/Engine/EditorBlueprintResources/StandardMacros.IsValid` (`self.Structure`)
        (:`Is Valid`
          (`Widget.RemoveFromParent` (`self.Structure`))
          (set `self.Structure` null)
          (`KismetSystemLibrary.Delay` 0.1)
          (bind _returnvalue (`|CreateWidget` "/Game/Game/UI/WB_Structure.WB_Structure_C"))
          (bind _output_get (set `self.Structure` _returnvalue))
          (`UserWidget.AddToViewport` _output_get 0)
          (`/Game/Game/UI/WB_Structure.Initialisation` _returnvalue Structure))
        (:`Is Not Valid`
          (bind _returnvalue_2 (`|CreateWidget` "/Game/Game/UI/WB_Structure.WB_Structure_C"))
          (bind _output_get_2 (set `self.Structure` _returnvalue_2))
          (`UserWidget.AddToViewport` _output_get_2 0)
          (`/Game/Game/UI/WB_Structure.Initialisation` _returnvalue_2 Structure))))))

(event `Load`
  (bind _returnvalue (`|CreateWidget` "/Game/Game/UI/WB_Load.WB_Load_C" null true))
  (bind _output_get (set `self.Loads` _returnvalue))
  (`UserWidget.AddToViewport` _output_get 0))

(event `Removes`
  (`Widget.RemoveFromParent` (`self.Loads`))
  (set `self.Loads` null))

(fn `UserConstructionScript`)