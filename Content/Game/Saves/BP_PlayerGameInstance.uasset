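; BP_PlayerGameInstance is a game instance that holds player state: stats, occupancy data, name and info.
; Init and Start share one path that seeds money, satisfaction and population stats from a starting data asset and sets Create to true.
; An Init event with parameters instead copies supplied stats, occupancy, name and info into the instance and clears Create, separating supplied state from fresh defaults.
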(event `self.ReceiveInit`
  (bind (_money _satisfaction _population _populationmax) (break `/Game/Game/Blueprints/DataAsset/S_StatsStart` (`/Game/Game/Blueprints/DataAsset/BP_DataAsset_StatsStart.Stats` (`self.DataAsset_StatsStart`))))
  (set `self.Stats` (make `/Game/Game/Blueprints/DataAsset/S_StatsStart` _money _satisfaction _population _populationmax) :!label _label)
  (set `self.Create` true))

(event `Start`
  (goto _label))

(event `Init`
  (params (Stats :type "/Game/Game/Blueprints/DataAsset/S_StatsStart Structure") (NewParam :type "Array of Boolean") (NewParam2 :type "Array of /Game/Game/Blueprints/Grid/E_BuildingType Enum") (NewParam3 :type "Array of Actor Object Reference") (NewParam4 :type "Array of String") (Info :type "Array of /Game/Game/Blueprints/DataAsset/S_Info Structure"))
  (set `self.Stats` Stats)
  (set `self.IsOccupied` NewParam)
  (set `self.OccupingType` NewParam2)
  (set `self.OccupingActor` NewParam3)
  (set `self.Name` NewParam4)
  (set `self.Info` Info)
  (set `self.Create` false))